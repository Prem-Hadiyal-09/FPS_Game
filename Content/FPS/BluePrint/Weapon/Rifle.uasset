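; Rifle weapon Blueprint for an FPS, handling firing, reloading and aim-down-sights.
; Its construction script fills WeaponData and a WeaponMaster struct of montages, sounds, effects and projectile, decal and shell classes.
; Fire, Reload and Ads delegate to WeaponComponent for ammo, line trace, muzzle flash, recoil and zoom, with an empty magazine triggering reload.
; Decal and shell calls are unwired, and a local AmmoCheck function goes uncalled here.
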(event EventAds
  (params (Alpha :type Float%20%28single-precision%29))
  (bind _weapondata (Variables|Default|GetWeaponData))
  (bind (_damage _feildofview _cameradistance) (Utilities|Struct|BreakWeaponData _weapondata))
  (Default|AdsBegin (Variables|Default|GetWeaponComponent) (Variables|Default|GetScope) Alpha _feildofview _cameradistance))

(event EventFire
  (if (> (.CurrentAmmo (Utilities|Struct|BreakWeaponData (Variables|Default|GetWeaponData))) 0)
    (Default|AmmoCheck (Variables|Default|GetWeaponComponent) (Variables|Default|GetWeapon) (.CurrentAmmo (Utilities|Struct|BreakWeaponData (Variables|Default|GetWeaponData))))
    (bind (_location _normal) (Default|LineTrace (Variables|Default|GetWeaponComponent) (Variables|Default|GetMuzzle) (.Spread (Utilities|Struct|BreakWeaponData (Variables|Default|GetWeaponData)))))
    (Default|FireBegin (Variables|Default|GetWeaponComponent))
    (Default|MuzzleFlash (Variables|Default|GetWeaponComponent) (Variables|Default|GetMuzzle))
    (Default|Recoil (Variables|Default|GetWeaponComponent) (.Recoil (Utilities|Struct|BreakWeaponData (Variables|Default|GetWeaponData))))
    (else
      (Default|EmptySFX (Variables|Default|GetWeaponComponent))
      (CallFunction|Reload))))

(event EventReload
  (bind _weapondata (Variables|Default|GetWeaponData))
  (bind (_currentammo _maxammo) (Utilities|Struct|BreakWeaponData _weapondata))
  (if (< _currentammo _maxammo)
    (Default|ReloadBegin (Variables|Default|GetWeaponComponent) (Variables|Default|GetWeapon) (.ReloadTime (Utilities|Struct|BreakWeaponData (Variables|Default|GetWeaponData))))))

(fn ConstructionScript
  (|CallParentFunction)
  (Variables|Default|SetWeaponData (Utilities|Struct|MakeWeaponData "Rifle_C" "NewEnumerator0" 30 30 2.7 1e+03 15.0 0.2 9e+01 3e+01 true "RifleSocket"))
  (Variables|Default|SetWeaponMaster (Utilities|Struct|MakeWeaponMaster (Utilities|Struct|MakeWeaponAnim "/Game/FPS/Animation/Arm/Rifle/Montage/Rifle_Fire_Montage.Rifle_Fire_Montage" "/Game/FPS/Animation/Weapon/Rifle/WeaponRifle_Fire_Montage.WeaponRifle_Fire_Montage" "/Game/FPS/Animation/Arm/Rifle/ADS/Rifle_FireADS_Montage.Rifle_FireADS_Montage" "/Game/FPS/Animation/Arm/Rifle/Montage/Rifle_Reload_Montage.Rifle_Reload_Montage" "/Game/FPS/Animation/Weapon/Rifle/WeaponRifle_Reload_Montage.WeaponRifle_Reload_Montage") (Utilities|Struct|MakeWeaponSFX "/Game/FPS/BluePrint/Weapon/SFX/Rifle_Cue.Rifle_Cue" "/Game/FPS/BluePrint/HUD/SFX/Empty.Empty") (Utilities|Struct|MakeWeaponVFX "/Game/MilitaryWeapDark/FX/P_AssaultRifle_MuzzleFlash.P_AssaultRifle_MuzzleFlash") (Utilities|Struct|MakeParticleSFX 0 "/Game/FPS/BluePrint/Weapon/VFX/Metal.Metal" "/Game/FPS/BluePrint/Weapon/VFX/Grass.Grass" "/Game/FPS/BluePrint/Weapon/VFX/Wood.Wood") (Utilities|Struct|MakeParticleVFX "/Game/MilitaryWeapDark/FX/P_SniperRifle_MuzzleFlash_01.P_SniperRifle_MuzzleFlash_01" "/Game/MilitaryWeapDark/FX/P_Impact_Metal_Medium_01.P_Impact_Metal_Medium_01" "/Game/MilitaryWeapDark/FX/P_Impact_Stone_Medium_01.P_Impact_Stone_Medium_01" "/Game/MilitaryWeapDark/FX/P_Impact_Wood_Medium_01.P_Impact_Wood_Medium_01") (Utilities|Struct|MakeWeaponClass "/Game/FPS/BluePrint/Bullet/Projectile/Rifle_Bullet.Rifle_Bullet_C" "/Game/FPS/BluePrint/Bullet/Decal/Decal.Decal_C" "/Game/FPS/BluePrint/Bullet/Shell/Rifle_Shell.Rifle_Shell_C"))))

(fn AmmoCheck
  (Math|Integer|DecrementInt (.CurrentAmmo (Utilities|Struct|BreakWeaponData (Variables|Default|GetWeaponData)))
    (:%20%20
      (|FireSFX)
      (if (not (Variables|/Game/FPS/BluePrint/FPS.FPS_C|GetisReload? (.AsFPS (Utilities|Casting|CastToFPS (Game|GetPlayerCharacter 0)))))
        (Components|Animation|PlayAnimation (Variables|Default|GetWeapon) "/Game/FPS/Animation/Weapon/Rifle/WeaponRifle_Fire.WeaponRifle_Fire" false)))))